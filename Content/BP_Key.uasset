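; BP_Key is a key pickup actor that the player collects by pressing E while inside its box trigger.
; Box overlap enables input on the actor, stores the overlapping BP_MainPlayer and shows a text prompt for three seconds; leaving the box disables input.
; Pressing E sets the player's KEYUP flag and destroys the key.
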(event `Key|E`
  (params (Key :type "Key Structure"))
  (:`Pressed`
    (set `/Game/BP_MainPlayer.kEY UP` true (stale `self.Box.OnComponentBeginOverlap` _asbp_main_player))
    (`self.K2_DestroyActor`)))

(event `self.Box.OnComponentBeginOverlap`
  (params (OverlappedComponent :type "PrimitiveComponent Object Reference") (OtherActor :type "Actor Object Reference") (OtherComp :type "PrimitiveComponent Object Reference") (OtherBodyIndex :type Integer) (bFromSweep :type Boolean) (SweepResult :type "HitResult Structure (by ref)"))
  (bind _textrender (`self.TextRender`))
  (`self.EnableInput` (`GameplayStatics.GetPlayerController` 0))
  (bind _asbp_main_player (cast `/Game/BP_MainPlayer` OtherActor))
  (`SceneComponent.SetVisibility` _textrender true false)
  (`KismetSystemLibrary.Delay` 3.0)
  (`SceneComponent.SetVisibility` _textrender false false))

(event `self.Box.OnComponentEndOverlap`
  (params (OverlappedComponent :type "PrimitiveComponent Object Reference") (OtherActor :type "Actor Object Reference") (OtherComp :type "PrimitiveComponent Object Reference") (OtherBodyIndex :type Integer))
  (`self.DisableInput` (`GameplayStatics.GetPlayerController` 0)))

(fn `UserConstructionScript`)